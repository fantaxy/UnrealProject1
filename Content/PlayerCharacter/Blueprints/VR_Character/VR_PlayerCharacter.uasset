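; VR player character Blueprint with trackpad locomotion, turning and two-handed object pickup through motion controllers.
; Input axes drive movement and view rotation, while grip and trigger keys set per-hand pressed flags.
; PickupObject attaches the passed object to the Vive controller mesh socket of each empty hand whose flag is set.
; Releasing either button on a hand detaches its held item and turns on physics simulation.
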(event `InputAxis|MoveForward`
  (params (AxisValue :type "Float (single-precision)"))
  ;[1 1 1] Trackpad Movement/Locomotion
  (`self.AddMovementInput` (`self.GetActorForwardVector`) AxisValue))

(event `Key|MotionController_Right_Grip1`
  (params (Key :type "Key Structure" :default "AnyKey"))
  ;[1 1 1] Pickup Object w/ Grip Buttons
  ; (Button Events could be Inputs instead if you wanted)
  (:`Pressed`
    (set `self.RightGripPressed` true :!label _label))
  (:`Released`
    (set `self.RightGripPressed` false :!label _label_2)
    (`self.DetachFromRightHand`)))

(event `Key|MotionController_Right_Trigger`
  (params (Key :type "Key Structure" :default "AnyKey"))
  ;[1 1 1] Pickup Object w/ Triggers
  ; (Trigger Events could be Inputs instead if you wanted)
  (:`Pressed`
    (set `self.RightTriggerPressed` true))
  (:`Released`
    (set `self.RightTriggerPressed` false)
    (`self.DetachFromRightHand`)))

(event `Key|MotionController_Right_Grip2`
  (params (Key :type "Key Structure" :default "AnyKey"))
  ;[1 1 1] Pickup Object w/ Grip Buttons
  ; (Button Events could be Inputs instead if you wanted)
  (:`Pressed`
    (goto _label))
  (:`Released`
    (goto _label_2)))

(event `InputAxis|MoveRight`
  (params (AxisValue :type "Float (single-precision)"))
  ;[1 1 1] Trackpad Movement/Locomotion
  (`self.AddMovementInput` (`self.GetActorRightVector`) AxisValue))

(event `Key|MotionController_Left_Grip1`
  (params (Key :type "Key Structure" :default "AnyKey"))
  ;[1 1 1] Pickup Object w/ Grip Buttons
  ; (Button Events could be Inputs instead if you wanted)
  (:`Pressed`
    (set `self.LeftGripPressed` true :!label _label_3))
  (:`Released`
    (set `self.LeftGripPressed` false :!label _label_4)
    (`self.DetachFromLeftHand`)))

(event `Key|MotionController_Left_Trigger`
  (params (Key :type "Key Structure" :default "AnyKey"))
  ;[1 1 1] Pickup Object w/ Triggers
  ; (Trigger Events could be Inputs instead if you wanted)
  (:`Pressed`
    (set `self.LeftTriggerPressed` true))
  (:`Released`
    (set `self.LeftTriggerPressed` false)
    (`self.DetachFromLeftHand`)))

(event `Key|MotionController_Left_Grip2`
  (params (Key :type "Key Structure" :default "AnyKey"))
  ;[1 1 1] Pickup Object w/ Grip Buttons
  ; (Button Events could be Inputs instead if you wanted)
  (:`Pressed`
    (goto _label_3))
  (:`Released`
    (goto _label_4)))

(event `InputAxis|TurnRate`
  (params (AxisValue :type "Float (single-precision)"))
  ;[1 1 1] Trackpad Turn Rate
  (`self.AddControllerYawInput` (* AxisValue (`self.BaseTurnRate`) (`GameplayStatics.GetWorldDeltaSeconds`))))

(event `/Game/Interfaces/PickUpObjectInterface.Pickup Object`
  (params (Object :type "StaticMeshActor Object Reference"))
  ;[1 1 1] Pickup Object
  (`self.RightHandPickup` Object) ; Custom Event
  (`self.LeftHandPickup` Object) ; Custom Event
)

(event `RightHandPickup`
  (params (ObjectToPickup :type "StaticMeshActor Object Reference"))
  ;[1 1 1] Pickup Object
  (if (or (`self.RightTriggerPressed`) (`self.RightGripPressed`))
    (`self.AttachToRightHand` ObjectToPickup)))

(event `InputAxis|LookUp`
  (params (AxisValue :type "Float (single-precision)"))
  (`self.AddControllerPitchInput` AxisValue))

(event `LeftHandPickup`
  (params (ObjectToPickup :type "StaticMeshActor Object Reference"))
  ;[1 1 1] Pickup Object
  (if (or (`self.LeftTriggerPressed`) (`self.LeftGripPressed`))
    (`self.AttachToLeftHand` ObjectToPickup)))

(event `InputAxis|Turn`
  (params (AxisValue :type "Float (single-precision)"))
  (`self.AddControllerYawInput` AxisValue))

(fn `AttachToLeftHand`
  (params (ObjectToPickup :type "StaticMeshActor Object Reference"))
  ;[1 1 1] Attach To Right Hand
  (if (== (`self.PickupItem2`) null)
    (`self.K2_AttachRootComponentTo` ObjectToPickup (`self.L_ViveMesh`) (`self.L_ViveMeshSocket`) (`self.AttachLocationType`) true) ; Specify any Socket or Attach Location as needed.
    (set `self.PickupItem2` ObjectToPickup))
  (return))

(fn `AttachToRightHand`
  (params (ObjectToPickup :type "StaticMeshActor Object Reference"))
  ;[1 1 1] Attach To Right Hand
  (if (== (`self.PickupItem`) null)
    (`self.K2_AttachRootComponentTo` ObjectToPickup (`self.R_ViveMesh`) (`self.R_ViveMeshSocket`) (`self.AttachLocationType`) true) ; Specify any Socket or Attach Location as needed.
    (set `self.PickupItem` ObjectToPickup))
  (return))

(fn `DetachFromLeftHand`
  (bind _pickupitem2 (`self.PickupItem2`))
  (if (!= (`self.PickupItem2`) null)
    (`self.DetachRootComponentFromParent` _pickupitem2 true)
    (`PrimitiveComponent.SetSimulatePhysics` (`StaticMeshActor.StaticMeshComponent` _pickupitem2) true)
    (set `self.PickupItem2` null))
  (return))

(fn `DetachFromRightHand`
  (bind _pickupitem (`self.PickupItem`))
  (if (!= (`self.PickupItem`) null)
    (`self.DetachRootComponentFromParent` _pickupitem true)
    (`PrimitiveComponent.SetSimulatePhysics` (`StaticMeshActor.StaticMeshComponent` _pickupitem) true)
    (set `self.PickupItem` null))
  (return))

(fn `UserConstructionScript`)